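; Functional test that checks whether BP_Ball's IsPlayerCharacter recognizes the player character.
; PrepareTest spawns a BP_Ball at the origin and stores it as TestBall.
; StartTest passes player character 0 to IsPlayerCharacter, asserts the result is true and finishes as succeeded or failed, though its result messages refer to a vector.
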(event `self.ReceivePrepareTest`
  (bind _returnvalue (`|SpawnActorFromClass` "/Game/Blueprints/Pitch/BP_Ball.BP_Ball_C" (`KismetMathLibrary.MakeTransform` (0.0 0.0 0.0)) "Undefined" "MultiplyWithRoot" null null))
  (set `self.TestBall` _returnvalue))

(event `self.ReceiveStartTest`
  (bind _returnvalue (`/Game/Blueprints/Pitch/BP_Ball.IsPlayerCharacter` (`self.TestBall`) (`GameplayStatics.GetPlayerCharacter` 0)))
  (bind _returnvalue_2 (`self.AssertTrue` _returnvalue))
  (if _returnvalue_2
    (`self.FinishTest` "Succeeded" "The vector was correct")
    (else
      (`self.FinishTest` "Failed" "The vector was incorrect"))))

(fn `UserConstructionScript`)