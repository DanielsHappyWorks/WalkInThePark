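; Functional test that checks setting a positive rotation on the Seesaw actor.
; PrepareTest spawns a Seesaw at the world origin and keeps a reference to it.
; StartTest sets a positive angle, reads the rotation back and asserts it matches the expected single-axis rotator, finishing as succeeded or failed.
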(event `self.ReceivePrepareTest`
  (bind _returnvalue (`|SpawnActorFromClass` "/Game/Blueprints/Park/Seesaw.Seesaw_C" (`KismetMathLibrary.MakeTransform` (0.0 0.0 0.0)) "Undefined" "MultiplyWithRoot" null null))
  (set `self.TestSeesaw` _returnvalue))

(event `self.ReceiveStartTest`
  (bind _testseesaw (`self.TestSeesaw`))
  (`/Game/Blueprints/Park/Seesaw.SetSeesawRotation` _testseesaw 18.0)
  (bind _rotation (`/Game/Blueprints/Park/Seesaw.GetSeesawRotation` _testseesaw))
  (bind _returnvalue (`self.AssertEqual_Rotator` _rotation (struct :`Pitch` 18.0)))
  (if _returnvalue
    (`self.FinishTest` "Succeeded" "The rotator was correct")
    (else
      (`self.FinishTest` "Failed" "The rotator was incorrect"))))

(fn `UserConstructionScript`)