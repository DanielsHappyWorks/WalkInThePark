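; Functional test that checks how BP_Water positions its mesh for a given alpha value.
; PrepareTest spawns a BP_Water at the world origin and asserts that its StaticMeshComponent starts there.
; StartTest calls SetNewLocationBasedOnTime with the Alpha variable and compares the mesh's world location to the expected vector.
; The final branch is hardwired true, so FinishTest always reports Succeeded, leaving any failure to the assertions.
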(event `self.ReceivePrepareTest`
  (bind _returnvalue (`|SpawnActorFromClass` "/Game/Blueprints/Lake/BP_Water.BP_Water_C" (`KismetMathLibrary.MakeTransform` (0.0 0.0 0.0)) "Undefined" "MultiplyWithRoot" null null))
  (set `self.Water` _returnvalue)
  (`self.AssertLocation` (0.0 0.0 0.0)))

(event `self.ReceiveStartTest`
  (`/Game/Blueprints/Lake/BP_Water.SetNewLocationBasedOnTime` (`self.Water`) (`self.Alpha`) (0.0 0.0 0.0))
  (`self.AssertLocation` (`self.Expecetd`))
  (if true
    (`self.FinishTest` "Succeeded")
    (else
      (`self.FinishTest` "Failed"))))

(fn `AssertLocation`
  (params (Expected :type "Vector Structure"))
  (returns (ReturnValue :type Boolean))
  (bind _returnvalue (`self.AssertEqual_Vector` (`SceneComponent.K2_GetComponentLocation` (`StaticMeshActor.StaticMeshComponent` (`self.Water`))) Expected))
  (return _returnvalue))

(fn `UserConstructionScript`)