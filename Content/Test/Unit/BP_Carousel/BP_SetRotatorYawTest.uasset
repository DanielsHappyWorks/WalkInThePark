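; Functional test that checks a Carousel's SetRotationRate correctly sets the yaw rate on its Rotator.
; PrepareTest spawns a Carousel at the origin and stores it as TestCarousel.
; StartTest sets the rate, compares the Rotator's RotationRate to the expected yaw-only rotator, and finishes as succeeded or failed.
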(event `self.ReceivePrepareTest`
  (bind _returnvalue (`|SpawnActorFromClass` "/Game/Blueprints/Park/Carousel.Carousel_C" (`KismetMathLibrary.MakeTransform` (0.0 0.0 0.0)) "Undefined" "MultiplyWithRoot" null null))
  (set `self.TestCarousel` _returnvalue))

(event `self.ReceiveStartTest`
  (bind _testcarousel (`self.TestCarousel`))
  (`/Game/Blueprints/Park/Carousel.SetRotationRate` _testcarousel 45.0)
  (bind _returnvalue (`self.AssertEqual_Rotator` (`RotatingMovementComponent.RotationRate` (`/Game/Blueprints/Park/Carousel.Rotator` _testcarousel)) (struct :`Yaw` 45.0)))
  (if _returnvalue
    (`self.FinishTest` "Succeeded" "The rotator was correct")
    (else
      (`self.FinishTest` "Failed" "The rotator was incorrect"))))

(fn `UserConstructionScript`)