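; Functional test that checks a Carousel actor rotates once given a rotation rate; the asset name says clockwise, but the direction is not asserted.
; PrepareTest spawns the carousel at the origin with zero rotation, and StartTest sets a positive rotation rate.
; A tick counter asserts the default rotation on the first frame, then finishes the test as succeeded once the rotation is no longer zero.
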(event `self.ReceivePrepareTest`
  (bind _returnvalue (`|SpawnActorFromClass` "/Game/Blueprints/Park/Carousel.Carousel_C" (`KismetMathLibrary.MakeTransform` (0.0 0.0 0.0)) "Undefined" "MultiplyWithRoot" null null))
  (set `self.TestCarousel` _returnvalue))

(event `self.ReceiveStartTest`
  (`/Game/Blueprints/Park/Carousel.SetRotationRate` (`self.TestCarousel`) 45.0))

(event `self.ReceiveTick`
  (params (DeltaSeconds :type "Float (single-precision)"))
  (bind _counter (`self.counter`))
  (bind _returnvalue (`self.K2_GetActorRotation` (`self.TestCarousel`)))
  (`/Engine/EditorBlueprintResources/StandardMacros.IncrementInt` _counter
    (:`  `
      (if (== _counter 1)
        (`self.AssertEqual_Rotator` _returnvalue)
        (else
          (bind _returnvalue_2 (`self.AssertNotEqual_Rotator` _returnvalue))
          (if _returnvalue_2
            (`self.FinishTest` "Succeeded")))))))

(fn `UserConstructionScript`)