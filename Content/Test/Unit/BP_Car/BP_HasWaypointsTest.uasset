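; Functional test that checks a car character reports having waypoints to walk to when it has been given one.
; PrepareTest spawns a BP_Waypoints and a BP_CarCharacter at the same location and sets the car's Waypoints array to that single waypoint.
; StartTest asserts HasWaypointsToWalkTo and finishes as succeeded or failed, though both result messages refer to a rotator rather than waypoints.
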(event `self.ReceivePrepareTest`
  (bind _returnvalue (`KismetMathLibrary.MakeTransform` (100.0 0.0 0.0)))
  (bind _returnvalue_2 (`|SpawnActorFromClass` "/Game/Blueprints/Citizens/BP_Waypoints.BP_Waypoints_C" _returnvalue "Undefined" "MultiplyWithRoot" null null))
  (bind _returnvalue_3 (`|SpawnActorFromClass` "/Game/Blueprints/Citizens/BP_CarCharacter.BP_CarCharacter_C" _returnvalue "Undefined" "MultiplyWithRoot" null null))
  (bind _output_get (set `self.Car` _returnvalue_3))
  (set `/Game/Blueprints/Citizens/BP_CitizenCharacter.Waypoints` (`|MakeArray` _returnvalue_2) _output_get))

(event `self.ReceiveStartTest`
  (bind _returnvalue (`/Game/Blueprints/Citizens/BP_CitizenCharacter.HasWaypointsToWalkTo` (`self.Car`)))
  (bind _returnvalue_2 (`self.AssertTrue` _returnvalue))
  (if _returnvalue_2
    (`self.FinishTest` "Succeeded" "The rotator was correct")
    (else
      (`self.FinishTest` "Failed" "The rotator was incorrect"))))

(fn `UserConstructionScript`)