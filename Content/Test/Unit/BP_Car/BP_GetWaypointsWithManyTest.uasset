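; Functional test that checks BP_CarCharacter's GetNextWaypoint cycles through a multi-entry waypoint list and wraps to the start.
; PrepareTest spawns a car at the origin and assigns it two spawned BP_Waypoints actors.
; StartTest calls the AssertNextWaypoint helper four times, expecting both waypoints in order, twice over.
; It then finishes through a hard-coded true branch as Succeeded, with a message that refers to a rotator.
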(event `self.ReceivePrepareTest`
  (bind (_returnvalue _returnvalue2) (`self.SpawnWaypoint`))
  (bind (_returnvalue_2 _returnvalue2_2) (`self.SpawnWaypoint`))
  (bind _returnvalue_3 (`|SpawnActorFromClass` "/Game/Blueprints/Citizens/BP_CarCharacter.BP_CarCharacter_C" (`KismetMathLibrary.MakeTransform` (0.0 0.0 0.0)) "Undefined" "MultiplyWithRoot" null null))
  (bind _output_get (set `self.Car` _returnvalue_3))
  (set `/Game/Blueprints/Citizens/BP_CitizenCharacter.Waypoints` (`|MakeArray` _returnvalue2 _returnvalue2_2) _output_get))

(event `self.ReceiveStartTest`
  ;[1 1 1] Will wrap back around after list is exhausted
  (`self.AssertNextWaypoint` (stale `self.ReceivePrepareTest` _returnvalue2))
  (`self.AssertNextWaypoint` (stale `self.ReceivePrepareTest` _returnvalue2_2))
  (`self.AssertNextWaypoint` (stale `self.ReceivePrepareTest` _returnvalue2))
  (`self.AssertNextWaypoint` (stale `self.ReceivePrepareTest` _returnvalue2_2))
  (if true
    (`self.FinishTest` "Succeeded" "The rotator was correct")
    (else
      (`self.FinishTest` "Failed" "The rotator was incorrect"))))

(fn `AssertNextWaypoint`
  (params (Expected :type "Object Object Reference"))
  (bind _output (`/Game/Blueprints/Citizens/BP_CitizenCharacter.getNextWaypoint` (`self.Car`)))
  (`self.AssertEqual_Object` _output Expected))

(fn `SpawnWaypoint`
  (returns (ReturnValue :type "Transform Structure") (ReturnValue2 :type "/Game/Blueprints/Citizens/BP_Waypoints Object Reference"))
  (bind _returnvalue (`KismetMathLibrary.MakeTransform` (100.0 0.0 0.0)))
  (bind _returnvalue_2 (`|SpawnActorFromClass` "/Game/Blueprints/Citizens/BP_Waypoints.BP_Waypoints_C" _returnvalue "Undefined" "MultiplyWithRoot" null null))
  (return _returnvalue _returnvalue_2))

(fn `UserConstructionScript`)