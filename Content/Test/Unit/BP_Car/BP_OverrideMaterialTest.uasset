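; Functional test that checks whether BP_CarCharacter applies its material override to the car's meshes.
; PrepareTest spawns a car character at the origin and assigns the test material as its MaterialOverride.
; StartTest calls OverrideMaterial, then compares material slot 0 on each direct child component of the BPCar child actor's root against the override.
; A mismatch or any non-static-mesh child fails the test; otherwise it succeeds.
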(event `self.ReceivePrepareTest`
  (bind _returnvalue (`|SpawnActorFromClass` "/Game/Blueprints/Citizens/BP_CarCharacter.BP_CarCharacter_C" (`KismetMathLibrary.MakeTransform` (0.0 0.0 0.0)) "Undefined" "MultiplyWithRoot" null null))
  (bind _output_get (set `self.Car` _returnvalue))
  (bind _output_get_2 (set `/Game/Blueprints/Citizens/BP_CarCharacter.MaterialOverride` (`self.Material`) _output_get)))

(event `self.ReceiveStartTest`
  (bind _car (`self.Car`))
  (`/Game/Blueprints/Citizens/BP_CarCharacter.OverrideMaterial` _car)
  (for _array_element (`SceneComponent.GetChildrenComponents` (`Actor.RootComponent` (`ChildActorComponent.ChildActor` (`/Game/Blueprints/Citizens/BP_CarCharacter.BP_Car` _car))) false)
    (bind _asstatic_mesh_component (cast `StaticMeshComponent` _array_element)
      (:`then`
        (bind _returnvalue (`self.AssertEqual_Object` (`PrimitiveComponent.GetMaterial` _asstatic_mesh_component 0) (stale `self.ReceivePrepareTest` _output_get_2)))
        (if (not _returnvalue)
          (`self.FinishTest` "Failed" :!label _label)))
      (:`CastFailed`
        (goto _label))))
  (`self.FinishTest` "Succeeded"))

(fn `UserConstructionScript`)