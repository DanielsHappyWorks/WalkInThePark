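; Functional test that checks a seesaw tilts fully to each side as the player character moves along it.
; Each tick it waits for the seesaw to reach its right-side limit, logging the rotation meanwhile.
; It then drives the character forward with movement input and succeeds once the left-side limit is reached.
; The seesaw overlap handler checks for the player but leaves the result unused.
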(event `self.ReceivePrepareTest`
  (set `self.Character` (`GameplayStatics.GetPlayerCharacter` 0)))

(event `self.ReceiveStartTest`)

(event `self.ReceiveTick`
  (params (DeltaSeconds :type "Float (single-precision)"))
  (if (`self.IsReachedBottom`)
    (`self.WalkToTheOtherSideOfTheSeesaw`)
    (`self.WaitForLeftSideToReachTheBottom`)
    (else
      (bind _returnvalue (`self.IsRightSideOfSeesawReachedTheBottom`))
      (set `self.IsReachedBottom` _returnvalue)
      (bind _rotation (`/Game/Blueprints/Park/Seesaw.GetSeesawRotation` (`self.Seesaw`)))
      (`KismetSystemLibrary.PrintString` (`KismetStringLibrary.Conv_RotatorToString` _rotation)))))

(event `self.Seesaw.OnActorBeginOverlap`
  (params (OverlappedActor :type "Actor Object Reference") (OtherActor :type "Actor Object Reference"))
  (`/Game/Blueprints/BP_Common.IsPlayerCharacter` OtherActor))

(fn `IsRightSideOfSeesawReachedTheBottom`
  (returns (ReturnValue :type Boolean))
  (bind _rotation (`/Game/Blueprints/Park/Seesaw.GetSeesawRotation` (`self.Seesaw`)))
  (return (== _rotation (struct :`Pitch` 18.0) :`ErrorTolerance` 0.0001)))

(fn `UserConstructionScript`)

(fn `WaitForLeftSideToReachTheBottom`
  (bind _rotation (`/Game/Blueprints/Park/Seesaw.GetSeesawRotation` (`self.Seesaw`)))
  (if (== _rotation (struct :`Pitch` -18.0) :`ErrorTolerance` 0.0001)
    (`self.AssertEqual_Rotator` _rotation (struct :`Pitch` -18.0))
    (`self.FinishTest` "Succeeded")))

(fn `WalkToTheOtherSideOfTheSeesaw`
  (bind _character (`self.Character`))
  (`Pawn.AddMovementInput` _character (`self.GetActorForwardVector` _character) 1.0 false))