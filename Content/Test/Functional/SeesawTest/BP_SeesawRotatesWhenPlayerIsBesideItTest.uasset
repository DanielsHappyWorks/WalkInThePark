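; Functional test that checks the seesaw rotates when the player is beside it.
; PrepareTest caches the player character, then Tick walks it forward and polls the seesaw's rotation.
; The test asserts and succeeds once the rotation matches the expected tilt within a small tolerance; the graph has no explicit failure branch.
; Helper functions for walking and checking either side reaching the bottom exist but are not called here.
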(event `self.ReceivePrepareTest`
  (set `self.Character` (`GameplayStatics.GetPlayerCharacter` 0)))

(event `self.ReceiveStartTest`)

(event `self.ReceiveTick`
  (params (DeltaSeconds :type "Float (single-precision)"))
  (bind _character (`self.Character`))
  (`Pawn.AddMovementInput` _character (`self.GetActorForwardVector` _character) 1.0 false)
  (bind _rotation (`/Game/Blueprints/Park/Seesaw.GetSeesawRotation` (`self.Seesaw`)))
  (if (== _rotation (struct :`Pitch` 18.0) :`ErrorTolerance` 0.0001)
    (`self.AssertEqual_Rotator` _rotation (struct :`Pitch` 18.0))
    (`self.FinishTest` "Succeeded")))

(fn `IsRightSideOfSeesawReachedTheBottom`
  (returns (ReturnValue :type Boolean))
  (bind _rotation (`/Game/Blueprints/Park/Seesaw.GetSeesawRotation` (`self.Seesaw`)))
  (return (== _rotation (struct :`Pitch` 18.0) :`ErrorTolerance` 0.0001)))

(fn `UserConstructionScript`)

(fn `WaitForLeftSideToReachTheBottom`
  (bind _rotation (`/Game/Blueprints/Park/Seesaw.GetSeesawRotation` (`self.Seesaw`)))
  (if (== _rotation (struct :`Pitch` -18.0) :`ErrorTolerance` 0.0001)
    (`self.AssertEqual_Rotator` _rotation (struct :`Pitch` -18.0))
    (`self.FinishTest` "Succeeded")))

(fn `WalkToTheOtherSideOfTheSeesaw`
  (bind _character (`self.Character`))
  (`Pawn.AddMovementInput` _character (`self.GetActorForwardVector` _character) 1.0 false))