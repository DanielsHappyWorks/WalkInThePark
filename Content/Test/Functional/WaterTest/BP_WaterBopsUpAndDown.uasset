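; Functional test that checks the Water actor bops up and down by alternately hitting two triggers, TriggerA and TriggerB.
; Each overlap increments CollisionCounter if the actor is Water, then asserts the counter's parity, odd for A and even for B, to enforce the order.
; The test finishes as succeeded when the counter equals 4, although the inline comment mentions five collisions.
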(event `self.TriggerA.OnActorBeginOverlap`
  (params (OverlappedActor :type "Actor Object Reference") (OtherActor :type "Actor Object Reference"))
  (`self.Increment Collision Count` OtherActor)
  ;[1 1 1] Check all triggers are hit in a specific order
  (`self.AssertCollidesInOrder` 1)
  ;[1 1 1] wait for 5 collisions before ending the test
  (if (== (`self.CollisionCounter`) 4) :!label _label
    (`self.FinishTest` "Succeeded")))

(event `self.TriggerB.OnActorBeginOverlap`
  (params (OverlappedActor :type "Actor Object Reference") (OtherActor :type "Actor Object Reference"))
  (`self.Increment Collision Count` OtherActor)
  ;[1 1 1] Check all triggers are hit in a specific order
  ;;[1 1 1] because we use %2 the assert looks for 0
  (`self.AssertCollidesInOrder` 0)
  (goto _label))

(fn `AssertCollidesInOrder`
  (params (Expected :type Integer))
  (returns (ReturnValue :type Boolean))
  (bind _returnvalue (`self.AssertEqual_Int` (mod (`self.CollisionCounter`) 2) Expected))
  (return _returnvalue))

(fn `Increment Collision Count`
  (params (A :type "Object Object Reference"))
  (returns (Result :type Integer))
  (if (== A (`self.water`))
    (bind _result (`/Engine/EditorBlueprintResources/StandardMacros.IncrementInt` (`self.CollisionCounter`))
      (:`  `
        (return _result)))))

(fn `UserConstructionScript`)