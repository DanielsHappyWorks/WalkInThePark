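; Functional test that checks the player character can kick a ball into a trigger.
; Caches the player character on prepare and drives it forward every tick with movement input.
; The test succeeds when the Ball actor begins overlapping the Trigger.
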(event `self.ReceivePrepareTest`
  (set `self.Character` (`GameplayStatics.GetPlayerCharacter` 0)))

(event `self.ReceiveStartTest`)

(event `self.ReceiveTick`
  (params (DeltaSeconds :type "Float (single-precision)"))
  (bind _character (`self.Character`))
  (`Pawn.AddMovementInput` _character (`self.GetActorForwardVector` _character) 1.0 false))

(event `self.Trigger.OnActorBeginOverlap`
  (params (OverlappedActor :type "Actor Object Reference") (OtherActor :type "Actor Object Reference"))
  (if (== OtherActor (`self.ball`))
    (`self.FinishTest` "Succeeded")))

(fn `UserConstructionScript`)