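; Functional test that checks a citizen walks around three triggers in repeating A, B, C order.
; Each trigger overlap increments a counter only for the Citizen, then asserts the counter modulo three matches that trigger's position, whichever actor overlapped.
; The test finishes as succeeded once the counter reaches five; the prepare, start and tick events are empty.
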(event `self.ReceivePrepareTest`)

(event `self.ReceiveStartTest`)

(event `self.ReceiveTick`
  (params (DeltaSeconds :type "Float (single-precision)")))

(event `ChectTestFinished`)

(event `self.TriggerA.OnActorBeginOverlap`
  (params (OverlappedActor :type "Actor Object Reference") (OtherActor :type "Actor Object Reference"))
  (`self.IncrementCollisionCounter` OtherActor)
  ;[1 1 1] Check all triggers are hit in a specific order
  (`self.AssertCollidesInOrder` 1)
  ;[1 1 1] wait for 5 collisions before ending the test
  (if (== (`self.CollisionCounter`) 5) :!label _label
    (`self.FinishTest` "Succeeded")))

(event `self.TriggerB.OnActorBeginOverlap`
  (params (OverlappedActor :type "Actor Object Reference") (OtherActor :type "Actor Object Reference"))
  (`self.IncrementCollisionCounter` OtherActor)
  ;[1 1 1] Check all triggers are hit in a specific order
  (`self.AssertCollidesInOrder` 2)
  (goto _label))

(event `self.TriggerC.OnActorBeginOverlap`
  (params (OverlappedActor :type "Actor Object Reference") (OtherActor :type "Actor Object Reference"))
  (`self.IncrementCollisionCounter` OtherActor)
  ;[1 1 1] Check all triggers are hit in a specific order
  ;;[1 1 1] because we use %3 the assert looks for 0
  (`self.AssertCollidesInOrder` 0)
  (goto _label))

(fn `AssertCollidesInOrder`
  (params (Expected :type Integer))
  (`self.AssertEqual_Int` (mod (`self.CollisionCounter`) 3) Expected))

(fn `IncrementCollisionCounter`
  (params (A :type "Object Object Reference"))
  (returns (Result :type Integer))
  (if (== A (`self.citizen`))
    (bind _result (`/Engine/EditorBlueprintResources/StandardMacros.IncrementInt` (`self.CollisionCounter`))
      (:`  `
        (return _result)))))

(fn `UserConstructionScript`)