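; Functional test that checks two citizens, CitizenA and CitizenB, each reach their own trigger, named for crossing paths.
; Overlaps on TriggerA and TriggerB increment a shared counter only when the overlapping actor is that trigger's assigned citizen.
; The test succeeds when the counter reaches two, without tracking which trigger contributed.
; An order-assertion helper based on the counter modulo three is defined but never called here.
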(event `self.TriggerA.OnActorBeginOverlap`
  (params (OverlappedActor :type "Actor Object Reference") (OtherActor :type "Actor Object Reference"))
  (`self.IncrementCollisionCounter` OtherActor (`self.citizenA`))
  (if (== (`self.CollisionCounter`) 2) :!label _label
    (`self.FinishTest` "Succeeded")))

(event `self.TriggerB.OnActorBeginOverlap`
  (params (OverlappedActor :type "Actor Object Reference") (OtherActor :type "Actor Object Reference"))
  (`self.IncrementCollisionCounter` OtherActor (`self.CitizenB`))
  (goto _label))

(fn `AssertCollidesInOrder`
  (params (Expected :type Integer))
  (`self.AssertEqual_Int` (mod (`self.CollisionCounter`) 3) Expected))

(fn `IncrementCollisionCounter`
  (params (Collision :type "Object Object Reference") (Citizen :type "Object Object Reference"))
  (returns (Result :type Integer))
  (if (== Collision Citizen)
    (bind _result (`/Engine/EditorBlueprintResources/StandardMacros.IncrementInt` (`self.CollisionCounter`))
      (:`  `
        (return _result)))))

(fn `UserConstructionScript`)