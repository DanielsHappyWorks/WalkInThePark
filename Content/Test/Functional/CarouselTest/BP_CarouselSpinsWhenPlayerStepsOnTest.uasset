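; Functional test that checks a carousel starts spinning when the player character steps onto it.
; Each tick before contact, it walks the character forward and asserts the carousel's rotation and Rotator speed are zero.
; The carousel's begin-overlap event flags player contact, switching Tick to poll the Rotator's rotation rate.
; The test succeeds once that rate exactly matches the expected maximum yaw or axis speed.
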(event `self.ReceivePrepareTest`
  (set `self.Character` (`GameplayStatics.GetPlayerCharacter` 0)))

(event `self.ReceiveStartTest`)

(event `self.ReceiveTick`
  (params (DeltaSeconds :type "Float (single-precision)"))
  (if (`self.IsCollididng`)
    (`self.WaitForMaxRotationSpeed`)
    (else
      (`self.StepOntoNotRotatingCarousel`))))

(event `self.Carousel.OnActorBeginOverlap`
  (params (OverlappedActor :type "Actor Object Reference") (OtherActor :type "Actor Object Reference"))
  (bind _returnvalue (`/Game/Blueprints/Common/BP_Common.IsPlayerCharacter` OtherActor))
  (set `self.IsCollididng` _returnvalue))

(fn `StepOntoNotRotatingCarousel`
  (bind _character (`self.Character`))
  (bind _carousel (`self.Carousel`))
  (`Pawn.AddMovementInput` _character (`self.GetActorForwardVector` _character) 1.0 false)
  (`self.AssertEqual_Rotator` (`self.K2_GetActorRotation` _carousel) (struct) "Carousel is not rotating")
  (`self.AssertEqual_Rotator` (`RotatingMovementComponent.RotationRate` (`/Game/Blueprints/Park/Carousel.Rotator` _carousel)) (struct) "Rotation speed is 0"))

(fn `UserConstructionScript`)

(fn `WaitForMaxRotationSpeed`
  (bind _rotationrate (`RotatingMovementComponent.RotationRate` (`/Game/Blueprints/Park/Carousel.Rotator` (`self.Carousel`))))
  (if (== _rotationrate (struct :`Yaw` -50.0))
    (`self.AssertEqual_Rotator` _rotationrate (struct :`Yaw` -50.0))
    (`self.FinishTest` "Succeeded")))