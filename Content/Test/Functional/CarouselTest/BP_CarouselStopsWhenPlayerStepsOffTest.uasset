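; Functional test checking that the carousel's rotation stops once the player steps off it.
; Tick polls the Carousel's Rotator until its RotationRate hits the hard-coded maximum.
; It then moves the player character backward with movement input each tick and succeeds when the rotation rate reaches zero.
; The test only observes the spin-up; its StartTest is empty and the overlap handler's player check drives nothing.
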(event `self.ReceivePrepareTest`
  (set `self.Character` (`GameplayStatics.GetPlayerCharacter` 0)))

(event `self.ReceiveStartTest`)

(event `self.ReceiveTick`
  (params (DeltaSeconds :type "Float (single-precision)"))
  (if (`self.IsMaxSpeed`)
    (`self.StepOffRotatingCarousel`)
    (`self.WaitForNoRotation`)
    (else
      (bind _returnvalue (`self.IsCarouselAtMaxRotation`))
      (set `self.IsMaxSpeed` _returnvalue))))

(event `self.Carousel.OnActorBeginOverlap`
  (params (OverlappedActor :type "Actor Object Reference") (OtherActor :type "Actor Object Reference"))
  (`/Game/Blueprints/Common/BP_Common.IsPlayerCharacter` OtherActor))

(fn `IsCarouselAtMaxRotation`
  (returns (ReturnValue :type Boolean))
  (return (== (`RotatingMovementComponent.RotationRate` (`/Game/Blueprints/Park/Carousel.Rotator` (`self.Carousel`))) (struct :`Yaw` -50.0))))

(fn `StepOffRotatingCarousel`
  (bind _character (`self.Character`))
  (`Pawn.AddMovementInput` _character (* (`self.GetActorForwardVector` _character) (-1.0 -1.0 -1.0)) 1.0 false))

(fn `UserConstructionScript`)

(fn `WaitForNoRotation`
  (bind _rotationrate (`RotatingMovementComponent.RotationRate` (`/Game/Blueprints/Park/Carousel.Rotator` (`self.Carousel`))))
  (if (== _rotationrate (struct))
    (`self.AssertEqual_Rotator` _rotationrate)
    (`self.FinishTest` "Succeeded")))