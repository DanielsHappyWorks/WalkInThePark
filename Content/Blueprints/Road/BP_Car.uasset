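; BP_Car is a road car Blueprint that manages the material on its child static meshes.
; OverRideMat loops over the direct children of DefaultSceneRoot and applies a given material to slot 0 of each static mesh.
; BeginPlay runs the same loop with no material assigned, which clears any slot 0 override.
; It contains no movement logic, and Tick is disabled.
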(event `self.ReceiveBeginPlay`
  (for _array_element (`SceneComponent.GetChildrenComponents` (`self.DefaultSceneRoot`) false)
    (bind _asstatic_mesh_component (cast `StaticMeshComponent` _array_element))
    (`PrimitiveComponent.SetMaterial` _asstatic_mesh_component 0 null)))

(fn `OverRideMat`
  (params (Material :type "MaterialInterface Object Reference"))
  (for _array_element (`SceneComponent.GetChildrenComponents` (`self.DefaultSceneRoot`) false)
    (bind _asstatic_mesh_component (cast `StaticMeshComponent` _array_element))
    (`PrimitiveComponent.SetMaterial` _asstatic_mesh_component 0 Material)))

(fn `UserConstructionScript`)