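; Park seesaw actor that tilts when the player character steps into the trigger on either side.
; Left trigger overlap plays a single Timeline forward and right trigger overlap reverses it, with its track driving the relative pitch of the SeesawUp component.
; Each valid overlap also requests a swinging sound cue, started only if not already playing.
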(event `self.ReceiveBeginPlay`)

(event `self.LeftTrigger.OnComponentBeginOverlap`
  (params (OverlappedComponent :type "PrimitiveComponent Object Reference") (OtherActor :type "Actor Object Reference") (OtherComp :type "PrimitiveComponent Object Reference") (OtherBodyIndex :type Integer) (bFromSweep :type Boolean) (SweepResult :type "HitResult Structure (by ref)"))
  (bind _returnvalue (`/Game/Blueprints/BP_Common.IsPlayerCharacter` OtherActor))
  (if _returnvalue
    (`/Game/Blueprints/BP_Audio.PlaySoundIfNotPlaying` (`self.Swinging_Cue`))
    ;[1 1 1] This cant be put in a function.
    ; See https://www.youtube.com/watch?v=w7lHw6zU51c
    (bind (_direction _newtrack_0) (`Timeline|Timeline` :!label _label)
      (:`Update`
        (`self.SetSeesawRotation` _newtrack_0)))))

(event `self.RightTrigger.OnComponentBeginOverlap`
  (params (OverlappedComponent :type "PrimitiveComponent Object Reference") (OtherActor :type "Actor Object Reference") (OtherComp :type "PrimitiveComponent Object Reference") (OtherBodyIndex :type Integer) (bFromSweep :type Boolean) (SweepResult :type "HitResult Structure (by ref)"))
  (bind _returnvalue (`/Game/Blueprints/BP_Common.IsPlayerCharacter` OtherActor))
  (if _returnvalue
    (`/Game/Blueprints/BP_Audio.PlaySoundIfNotPlaying` (`self.Swinging_Cue`))
    (goto _label :!via `Reverse`)))

(fn `GetSeesawRotation`
  (returns (Rotation :type "Rotator Structure"))
  (return (`SceneComponent.RelativeRotation` (`self.seesaw_up`))))

(fn `SetSeesawRotation`
  (params (Pitch :type "Float (single-precision)"))
  (`SceneComponent.K2_SetRelativeRotation` (`self.seesaw_up`) (`KismetMathLibrary.MakeRotator` 0.0 Pitch) false false))

(fn `UserConstructionScript`)