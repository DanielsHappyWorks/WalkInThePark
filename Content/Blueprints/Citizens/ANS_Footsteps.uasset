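; Animation notify for citizens that plays a footstep sound matching the surface under the character.
; On notify, it line traces on the Visibility channel from the mesh owner's location 200 units along its down vector.
; On a hit, the physical surface type selects a pavement, grass, gravel, bridge (wood) or swimming (water) cue, defaulting to pavement.
; The cue plays at the trace's end point rather than the impact point.
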(fn `GetLineTraceLocation`
  (params (actor :type "ActorComponent Object Reference"))
  (returns (Start :type "Vector Structure") (End :type "Vector Structure"))
  (bind _returnvalue (`ActorComponent.GetOwner` actor))
  (bind _returnvalue_2 (`Actor.K2_GetActorLocation` _returnvalue))
  (return _returnvalue_2 (+ _returnvalue_2 (* (`Actor.GetActorUpVector` _returnvalue) -200.0))))

(fn `PlayFootstepBasedOnMaterial`
  (params (Selection :type "EPhysicalSurface Enum" :default "SurfaceType_Default") (Location :type "Vector Structure"))
  (switch `EPhysicalSurface` Selection
    (:`SurfaceType_Default`
      (`GameplayStatics.PlaySoundAtLocation` "/Game/Sounds/Produced/Footsteps/Cues/Pavement_Cue.Pavement_Cue" Location (struct) 1.0 1.0 0.0 null null null null :!label _label))
    (:`SurfaceType1`
      (goto _label))
    (:`SurfaceType2`
      (`GameplayStatics.PlaySoundAtLocation` "/Game/Sounds/Produced/Footsteps/Cues/Grass_Cue.Grass_Cue" Location (struct) 1.0 1.0 0.0 null null null null))
    (:`SurfaceType3`
      (`GameplayStatics.PlaySoundAtLocation` "/Game/Sounds/Produced/Footsteps/Cues/Gravel_Cue.Gravel_Cue" Location (struct) 1.0 1.0 0.0 null null null null))
    (:`SurfaceType4`
      (`GameplayStatics.PlaySoundAtLocation` "/Game/Sounds/Produced/Footsteps/Cues/Bridge_Cue.Bridge_Cue" Location (struct) 1.0 1.0 0.0 null null null null))
    (:`SurfaceType5`
      (`GameplayStatics.PlaySoundAtLocation` "/Game/Sounds/Sourced/Swimming/Swimming_Cue.Swimming_Cue" Location (struct) 1.0 1.0 0.0 null null null null))))

(fn `Received_Notify`
  (params (MeshComp :type "SkeletalMeshComponent Object Reference") (Animation :type "AnimSequenceBase Object Reference") (EventReference :type "AnimNotifyEventReference Structure (by ref)"))
  (returns (ReturnValue :type Boolean))
  ;[1 1 1] See toutorial: https://www.youtube.com/watch?v=4tVMdNEOUNE
  ; Had to fix multiple issues including attenuation support myself
  (bind (_start _end) (`self.GetLineTraceLocation` MeshComp))
  (bind (_outhit _returnvalue) (`KismetSystemLibrary.LineTraceSingle` _start _end "TraceTypeQuery1"))
  (if _returnvalue
    (`self.PlayFootstepBasedOnMaterial` (`GameplayStatics.GetSurfaceType` _outhit) _end)
    (return _returnvalue)))