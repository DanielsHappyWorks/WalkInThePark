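; Citizen character that endlessly patrols a list of waypoint actors using AI navigation.
; On BeginPlay it sends AI MoveTo to the next waypoint and calls itself again when the move finishes.
; A wrapping counter loops back to the first waypoint after the last.
; A failed move or empty waypoint list only prints a debug message, and a failed move is not retried.
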(event `self.ReceiveBeginPlay`
  (`self.WalkToNextWaypoint`))

(event `WalkToNextWaypoint`
  (bind _returnvalue (`self.HasWaypointsToWalkTo`))
  (if _returnvalue
    (bind _output (`self.getNextWaypoint`))
    (`AITask_MoveTo.AIMoveTo` (`AIBlueprintHelperLibrary.GetAIController` self) (0.0 0.0 0.0) _output
      (:`OnRequestFailed`
        (`KismetSystemLibrary.PrintString` "Citizen Failed"))
      (:`OnMoveFinished`
        (`self.WalkToNextWaypoint`)))
    (else
      (`KismetSystemLibrary.PrintString` "Citizen Has no waypoints"))))

(fn `getNextWaypoint`
  (returns (Output :type "/Game/Blueprints/Citizens/BP_Waypoints Object Reference"))
  (locals (`Next Waypoint` :type "/Game/Blueprints/Citizens/BP_Waypoints Object Reference"))
  (bind _output_get (set `local.Next Waypoint` (`|GetArrayItem` (`self.Waypoints`) (`self.WaypointCounter`))))
  (`self.PointCounterAtNextWaypoint`)
  (return _output_get))

(fn `HasWaypointsToWalkTo`
  (returns (ReturnValue :type Boolean))
  (return (!= (`KismetArrayLibrary.Array_Length` (`self.Waypoints`)) 0)))

(fn `IsCounterAtLastWaypoint`
  (returns (ReturnValue :type Boolean))
  (return (== (+ (`self.WaypointCounter`) 1) (`KismetArrayLibrary.Array_Length` (`self.Waypoints`)))))

(fn `PointCounterAtNextWaypoint`
  (returns (Result :type Integer))
  (bind _returnvalue (`self.IsCounterAtLastWaypoint`))
  (if _returnvalue
    (bind _output_get (set `self.WaypointCounter` 0))
    (return _output_get)
    (else
      (bind _result (`/Engine/EditorBlueprintResources/StandardMacros.IncrementInt` (`self.WaypointCounter`))
        (:`  `
          (return _result))))))

(fn `UserConstructionScript`)