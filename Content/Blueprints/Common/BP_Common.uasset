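; BP_Common is a set of shared helper functions for working with the player character at index 0.
; IsPlayerCharacter tests whether an object is that character, and GetPlayerForwardVector returns the forward vector of its actor rotation.
; LaunchPlayer launches it with a given velocity, replacing vertical velocity while adding to horizontal velocity.
; A cast to BP_FirstPersonCharacter sits unconnected in IsPlayerCharacter and never runs.
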(fn `GetPlayerForwardVector`
  (returns (ReturnValue :type "Vector Structure"))
  (return (`KismetMathLibrary.GetForwardVector` (`Actor.K2_GetActorRotation` (`GameplayStatics.GetPlayerCharacter` null)))))

(fn `IsPlayerCharacter`
  (params (Object :type "Object Object Reference"))
  (returns (ReturnValue :type Boolean))
  (return (== Object (`GameplayStatics.GetPlayerCharacter` null))))

(fn `LaunchPlayer`
  (params (LaunchVelocity :type "Vector Structure"))
  (`Character.LaunchCharacter` (`GameplayStatics.GetPlayerCharacter` null) LaunchVelocity false true))