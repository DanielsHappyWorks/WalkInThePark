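; Soccer ball actor for the pitch that gets kicked when the player character runs into it.
; A component hit by the player triggers KickBall, which plays a kick sound if not already playing.
; The kick applies a velocity-change impulse along the player's horizontal forward direction, scaled by ForwardImpulse, with a fixed UpwardImpulse for lift.
; Bounce sound logic is unfinished and never runs.
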(event `self.soccer_ball.OnComponentHit`
  (params (HitComponent :type "PrimitiveComponent Object Reference") (OtherActor :type "Actor Object Reference") (OtherComp :type "PrimitiveComponent Object Reference") (NormalImpulse :type "Vector Structure") (Hit :type "HitResult Structure (by ref)"))
  (bind _returnvalue (`/Game/Blueprints/BP_Common.IsPlayerCharacter` OtherActor))
  (if _returnvalue
    (`self.KickBall`)))

(fn `CalculateImpulseVector`
  (params (NormalVector :type "Vector Structure"))
  (returns (ImpulseInVectorDirection :type "Vector Structure"))
  (bind _forwardimpulse (`self.ForwardImpulse`))
  (return (`KismetMathLibrary.MakeVector` (* (.x NormalVector) _forwardimpulse) (* (.y NormalVector) _forwardimpulse) (`self.UpwardImpulse`))))

(fn `KickBall`
  (`/Game/Blueprints/BP_Audio.PlaySoundIfNotPlaying` (`self.BallKick_Cue`))
  (bind _returnvalue (`/Game/Blueprints/BP_Common.GetPlayerForwardVector`))
  (bind _impulseinvectordirection (`self.CalculateImpulseVector` _returnvalue))
  (`PrimitiveComponent.AddImpulse` (`self.soccer_ball`) _impulseinvectordirection "None" true))

(fn `UserConstructionScript`)